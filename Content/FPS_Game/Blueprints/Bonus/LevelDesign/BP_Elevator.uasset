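; BP_Elevator is an interactable elevator that moves its floor between a down and an up position.
; Each BPIInteraction event toggles NextIndex and plays or reverses a Timeline, whose Alpha lerps the floor's relative location between ElevatorDown and ElevatorUp.
; BeginPlay applies ElevatorSpeed as the play rate and uses ElevatorStartsUp to set the starting position, toggle state and Timeline time, with a hardcoded 5.0 for the up state.
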(event `/Game/FPS_Game/Blueprints/System/BPI_Interact.BPI_Interaction`
  (params (CharacterReference :type "/Game/FPS_Game/Blueprints/BP_CharacterBase Object Reference"))
  (switch `int` (`self.Next Index`)
    (:`Default`
      (set `self.Next Index` 1 :!label _label)
      (bind (_direction _alpha) (`Timeline|Timeline` :!label _label_2)
        (:`Update`
          (`SceneComponent.K2_SetRelativeLocation` (`self.Floor`) (`KismetMathLibrary.VLerp` (`self.Elevator_Down`) (`self.Elevator_Up`) _alpha) false false))))
    (:`0`
      (goto _label))
    (:`1`
      (set `self.Next Index` 0)
      (goto _label_2 :!via `Reverse`))))

(event `self.ReceiveBeginPlay`
  (bind _elevator_starts_up (`self.Elevator Starts Up`))
  ; Set Elevator configurations
  (`TimelineComponent.SetPlayRate` (`self.Timeline`) (`self.Elevator Speed`))
  (set `self.Next Index` (`KismetMathLibrary.Conv_BoolToInt` _elevator_starts_up))
  (if _elevator_starts_up
    (`SceneComponent.K2_SetRelativeLocation` (`self.Floor`) (`self.Elevator_Up`) false false)
    (else
      (`SceneComponent.K2_SetRelativeLocation` (`self.Floor`) (`self.Elevator_Down`) false false)))
  (`TimelineComponent.SetNewTime` (`self.Timeline`) (* (`self.Elevator Starts Up`) 5.0)))

(fn `UserConstructionScript`)